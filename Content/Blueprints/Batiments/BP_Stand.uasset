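; BP_Stand is a building that hands out tools by spawning a ToolToGive actor each time it levels up.
; It keeps Box overlaps off until the first BP_Base fires its upgradable dispatcher, then enables them and sets the stand mesh.
; LevelUp spawns tools up to MaxNumberOfTools, resetting CoinsStocker and updating BatimentUI each time.
; CalculateSpawnPos is a stub with an empty loop, always returning the zero vector.
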(event Custom|EventInitStand
  (Variables|/Script/Engine.PrimitiveComponent|SetbGenerateOverlapEvents (Variables|Default|GetBox) true)
  (Components|StaticMesh|SetStaticMesh (Variables|Default|GetStaticMesh) "/Game/Level/_GENERATED/jujul/Stand.Stand"))

(event EventBeginPlay
  (|CallParentFunction)
  (Variables|/Script/Engine.PrimitiveComponent|SetbGenerateOverlapEvents (Variables|Default|GetBox) false)
  (bind _outactors (Actor|GetAllActorsOfClass "/Game/Blueprints/Batiments/BP_Base.BP_Base_C"))
  (bind _output_get (Variables|Default|SetBaseRef (Utilities|Array|Get(acopy) _outactors)))
  (EventDispatchers|BindEventtoEDUpgradable _output_get (delegate Custom|EventInitStand))
  (Variables|Default|SetNumberOfTool 0))

(fn ConstructionScript
  (|CallParentFunction))

(fn LevelUp
  (params (LevelDown :type Boolean))
  (if (not (== (Variables|Default|GetNumberOfTool) (Variables|Default|GetMaxNumberOfTools)))
    (bind _postion (CallFunction|CalculateSpawnPos))
    (Game|SpawnActorfromClass (Variables|Default|GetToolToGive) (Math|Transform|MakeTransform _postion "0, 0, 0" "1.000000,1.000000,1.000000") "AdjustIfPossibleButAlwaysSpawn" "MultiplyWithRoot" 0 0)
    (Variables|Default|SetCoinsStocker 0)
    (CallFunction|FunctionSetUI (Variables|Default|GetBatiment%20UI) false)
    (bind _result (Math|Integer|IncrementInt (Variables|Default|GetNumberOfTool))
      (:%20%20
        (Variables|Default|SetNumberOfTool _result)))))

(fn CalculateSpawnPos
  (for _index (range 0 (Variables|Default|GetMaxNumberOfTools))
    _)
  (return "0, 0, 0"))