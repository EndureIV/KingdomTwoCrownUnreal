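; BP_FireCamp is a campfire building that keeps up to two "Mandiant" BP_IA characters wandering around it.
; At BeginPlay and on the player character's new-day event, it fills empty slots during daytime, spawning AI with a wander area centred on CenterSpawn.
; Each AI's "remove from firecamp influence" dispatcher clears its slot, so a later spawn pass can replace it.
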(event Custom|EventDeletMandiant1
  (Variables|Default|SetMandiant1 0))

(event Custom|EventDeletMandiant2
  (Variables|Default|SetMandiant2 0))

(event Custom|EventSpawn
  (bind _mandiant1 (Variables|Default|GetMandiant1))
  (bind _mandiant2 (Variables|Default|GetMandiant2))
  (for _index (range 0 1)
    (CallFunction|Spawn))
  (Utilities|IsValid _mandiant1
    (:Is%20Valid
      (EventDispatchers|BindEventtoEDRemovefromFirecampInfluence _mandiant1 (delegate Custom|EventDeletMandiant1))
      (Utilities|IsValid _mandiant2
        (:Is%20Valid
          (EventDispatchers|BindEventtoEDRemovefromFirecampInfluence _mandiant2 (delegate Custom|EventDeletMandiant2)))))))

(event EventBeginPlay
  (bind _asbp_character (Utilities|Casting|CastToBP_Character (Game|Player|GetPlayerPawn 0)))
  (bind _output_get (Variables|Default|SetCharater _asbp_character))
  (EventDispatchers|AssignEDANewDay _output_get (delegate Custom|EventSpawn))
  (CallFunction|EventSpawn))

(fn ConstructionScript)

(fn Spawn
  (if (Variables|/Game/Blueprints/BP_Character.BP_Character_C|GetIsDay (Variables|Default|GetCharater))
    (if (== (Variables|Default|GetMandiant1) 0)
      (bind _returnvalue (Game|SpawnActorfromClass "/Game/Blueprints/IA/PNJ/BP_IA.BP_IA_C" (Utilities|LocationSpawn) "AdjustIfPossibleButAlwaysSpawn" "MultiplyWithRoot" 0 0))
      (bind _output_get (Variables|Default|SetMandiant1 _returnvalue))
      (Variables|/Game/Blueprints/IA/PNJ/BP_IA.BP_IA_C|SetCenterWanderPos _output_get (Transformation|GetWorldLocation (Variables|Default|GetCenterSpawn)))
      (Variables|/Game/Blueprints/IA/PNJ/BP_IA.BP_IA_C|SetWanderRadius _output_get 4e+02)
      (elif (== (Variables|Default|GetMandiant2) 0)
        (bind _returnvalue_2 (Game|SpawnActorfromClass "/Game/Blueprints/IA/PNJ/BP_IA.BP_IA_C" (Utilities|LocationSpawn) "AdjustIfPossibleButAlwaysSpawn" "MultiplyWithRoot" 0 0))
        (bind _output_get_2 (Variables|Default|SetMandiant2 _returnvalue_2))
        (Variables|/Game/Blueprints/IA/PNJ/BP_IA.BP_IA_C|SetCenterWanderPos _output_get_2 (Transformation|GetWorldLocation (Variables|Default|GetCenterSpawn)))
        (Variables|/Game/Blueprints/IA/PNJ/BP_IA.BP_IA_C|SetWanderRadius _output_get_2 4e+02)))))