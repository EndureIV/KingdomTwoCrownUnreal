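; BP_Batiments is a building the player upgrades by paying coins while standing in its overlap box, which also shows its cost widget.
; The character's pay event deposits one coin at a time, levelling up when the linearly rising cost is met, until max level.
; When paying stops, stored coins are dropped back through the character.
; Sounds and BPW_BatimentUI updates give feedback.
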(event OnComponentBeginOverlap(Box)
  (params (OverlappedComponent :type Primitive%20Component%20Object%20Reference) (OtherActor :type Actor%20Object%20Reference) (OtherComp :type Primitive%20Component%20Object%20Reference) (OtherBodyIndex :type Integer) (bFromSweep :type Boolean) (SweepResult :type Hit%20Result%20Structure%20%28by%20ref%29))
  (CallFunction|SetVisbilityWidget OtherActor true)
  (Variables|Default|SetOverlapPlayer true))

(event OnComponentEndOverlap(Box)
  (params (OverlappedComponent :type Primitive%20Component%20Object%20Reference) (OtherActor :type Actor%20Object%20Reference) (OtherComp :type Primitive%20Component%20Object%20Reference) (OtherBodyIndex :type Integer))
  (CallFunction|SetVisbilityWidget OtherActor false)
  (Variables|Default|SetOverlapPlayer false))

(event Custom|EventPay
  (CallFunction|Pay))

(event Custom|EventStopPaying
  (for _index (range 0 (- (Variables|Default|GetCoinsStocker) 1))
    (Default|DropCoins (Variables|Default|GetAs%20BP%20Character)))
  (Variables|Default|SetCoinsStocker 0)
  (Utilities|SetUI (Variables|Default|GetAs%20BPW%20Batiment%20UI)))

(event EventBeginPlay
  (bind _asbpw_batiment_ui (Utilities|Casting|CastToBPW_BatimentUI (UserInterface|GetWidget (Variables|Default|GetWidget))))
  (bind _output_get (Variables|Default|SetAs%20BPW%20Batiment%20UI _asbpw_batiment_ui))
  (Utilities|SetUI _output_get
    (:out
      (bind _asbp_character (Utilities|Casting|CastToBP_Character (Game|Player|GetPlayerPawn 0)))
      (bind _output_get_2 (Variables|Default|SetAs%20BP%20Character _asbp_character))
      (EventDispatchers|BindEventtoEDPay _output_get_2 (delegate Custom|EventPay))
      (EventDispatchers|BindEventtoEDStopPaying _output_get_2 (delegate Custom|EventStopPaying)))))

(fn ConstructionScript)

(fn LevelUp
  (if (not (== (Variables|Default|GetCurrentLevel) (Variables|Default|GetMaxLevel)))
    (bind _result (Math|Integer|IncrementInt (Variables|Default|GetCurrentLevel))
      (:%20%20
        (Variables|Default|SetCurrentLevel _result)
        (Variables|Default|SetCoinsStocker 0)
        (CallFunction|SetCostLevelUp (Variables|Default|GetBaseCost) (Variables|Default|GetIncreaseCost))))))

(fn SetCostLevelUp
  (params (BaseCost :type Integer) (Increase :type Integer))
  (Variables|Default|SetCostToLevelUp (+ BaseCost (* Increase (Variables|Default|GetCurrentLevel)))))

(fn SetVisbilityWidget
  (params (Object :type Object%20Object%20Reference) (Visibility :type Boolean))
  (Utilities|Casting|CastToBP_Character Object)
  (Rendering|SetVisibility (Variables|Default|GetWidget) Visibility false))

(fn Pay
  (if (Variables|Default|GetOverlapPlayer)
    (if (and (< (Variables|Default|GetCurrentLevel) (Variables|Default|GetMaxLevel)) (< (Variables|Default|GetCoinsStocker) (Variables|Default|GetCostToLevelUp)))
      (bind _result (Math|Integer|IncrementInt (Variables|Default|GetCoinsStocker))
        (:%20%20
          (Variables|Default|SetCoinsStocker _result)
          (Utilities|SetUI (Variables|Default|GetAs%20BPW%20Batiment%20UI)
            (:out
              (Audio|PlaySound2D "/Game/Sounds/CoinPerdu.CoinPerdu" 1.0 1.0 0.0 0 0)
              (CallFunction|AttemptLevelUp)))))
      (else
        (Audio|PlaySound2D "/Game/Sounds/Denied.Denied" 1.0 1.0 0.0 0 0)))))

(fn AttemptLevelUp
  (if (== (Variables|Default|GetCoinsStocker) (Variables|Default|GetCostToLevelUp))
    (CallFunction|LevelUp)
    (Audio|PlaySound2D "/Game/Sounds/Upgrade.Upgrade" 1.0 1.0 0.0 0 0)
    (Utilities|SetUI (Variables|Default|GetAs%20BPW%20Batiment%20UI))))