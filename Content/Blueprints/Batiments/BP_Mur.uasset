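; Wall building Blueprint that extends a parent class providing leveling and hit point data.
; LevelUp runs the parent logic, then restores CurrentHP to MaxHP.
; Tick prints CurrentHP on screen every frame as a debug readout, while BeginPlay and the construction script only call their parent versions.
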(event EventBeginPlay
  (|CallParentFunction))

(event EventTick
  (params (DeltaSeconds :type Float%20%28single-precision%29))
  (Development|PrintString (Utilities|String|ToString(Integer) (Variables|Default|GetCurrentHP)) true true "(R=0.000000,G=0.660000,B=1.000000,A=1.000000)" DeltaSeconds))

(fn ConstructionScript
  (|CallParentFunction))

(fn LevelUp
  (|CallParentFunction)
  (Variables|Default|SetCurrentHP (Variables|Default|GetMaxHP)))