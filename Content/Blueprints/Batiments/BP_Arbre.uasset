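; BP_Arbre is a tree actor in the buildings folder, tracked by its base as a destructible tree.
; On BeginPlay it runs the parent logic, then disables overlap events on its Box through ActivateBox, which can switch them back on.
; LevelUp removes the tree from the base's ArbreDestructibe collection and destroys the actor, so levelling up clears the tree.
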(event EventBeginPlay
  (|CallParentFunction)
  (CallFunction|ActivateBox false))

(fn ConstructionScript
  (|CallParentFunction))

(fn LevelUp
  (Utilities|Array|RemoveItem (Variables|/Game/Blueprints/Batiments/BP_Base.BP_Base_C|GetArbreDestructibe (Variables|Default|GetBaseRef)) self)
  (Actor|DestroyActor))

(fn ActivateBox
  (params (Generate%20Overlap%20Events :type Boolean))
  (Variables|/Script/Engine.PrimitiveComponent|SetbGenerateOverlapEvents (Variables|Default|GetBox) Generate%20Overlap%20Events))