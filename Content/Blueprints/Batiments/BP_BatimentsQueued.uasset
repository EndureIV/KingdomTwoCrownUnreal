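; Building Blueprint whose level-up is queued on the BP_Base instead of being applied directly.
; On BeginPlay it caches the first BP_Base and turns off overlap events on its collision box.
; AttemptLevelUp, once stored coins equal the cost, appends the building to the base's construction array, plays a sound, updates its UI, deactivates collision and flags it as upgrading.
; The preceding duplicate scan only breaks the loop, with the append following it.
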(event EventBeginPlay
  (|CallParentFunction)
  (bind _outactors (Actor|GetAllActorsOfClass "/Game/Blueprints/Batiments/BP_Base.BP_Base_C"))
  (Variables|Default|SetBaseRef (Utilities|Array|Get(acopy) _outactors))
  (CallFunction|SetActiveBox false))

(fn ConstructionScript
  (|CallParentFunction))

(fn AttemptLevelUp
  (bind _self self)
  (bind _baseref (Variables|Default|GetBaseRef))
  (bind _arrayconstruction (Variables|/Game/Blueprints/Batiments/BP_Base.BP_Base_C|GetArrayConstruction _baseref))
  (if (== (Variables|Default|GetCoinsStocker) (Variables|Default|GetCostToLevelUp))
    (bind _array_element (Utilities|Array|ForEachLoopwithBreak _arrayconstruction :!label _label)
      (:LoopBody
        (if (== _array_element _self)
          (goto _label Break)))
      (:Completed
        (Utilities|Array|Add _arrayconstruction _self)
        (Audio|PlaySound2D "/Game/Sounds/CoinRamasser.CoinRamasser" 1.0 1.0 0.0 0 0)
        (CallFunction|FunctionSetUI (Variables|Default|GetBatiment%20UI) false)
        (Components|Activation|SetActive (Variables|Default|GetCollisionBox) false false)
        (Variables|Default|SetIsCurrentlyUpgraded true)))))

(fn SetActiveBox
  (params (Generate%20Overlap%20Events :type Boolean))
  (Variables|/Script/Engine.PrimitiveComponent|SetbGenerateOverlapEvents (Variables|Default|GetCollisionBox) Generate%20Overlap%20Events))