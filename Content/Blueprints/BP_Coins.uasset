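; BP_Coins is a coin pickup that adds one coin to the BP_Character that overlaps it.
; Two seconds after BeginPlay, its Sphere component switches to overlap on a custom game trace channel.
; An overlap with a BP_Character calls AddCoins and destroys the actor.
; A separate SelfDestroy event, not called within this Blueprint, destroys the coin after a short random delay.
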(event OnComponentBeginOverlap(Sphere)
  (params (OverlappedComponent :type Primitive%20Component%20Object%20Reference) (OtherActor :type Actor%20Object%20Reference) (OtherComp :type Primitive%20Component%20Object%20Reference) (OtherBodyIndex :type Integer) (bFromSweep :type Boolean) (SweepResult :type Hit%20Result%20Structure%20%28by%20ref%29))
  (bind _asbp_character (Utilities|Casting|CastToBP_Character OtherActor))
  (Default|AddCoins _asbp_character 1)
  (Actor|DestroyActor))

(event Custom|SelfDestroy
  (Utilities|FlowControl|Delay (Math|Random|RandomFloatinRange 0.5 0.9))
  (Actor|DestroyActor))

(event EventBeginPlay
  (Utilities|FlowControl|Delay 2.0)
  (Collision|SetCollisionResponsetoChannel (Variables|Default|GetSphere) "ECC_GameTraceChannel1" "ECR_Overlap"))

(fn ConstructionScript)