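; BP_Batiments is a building actor that gains a level when the player character enters its trigger box.
; BeginPlay starts it at level zero with a cap, and the Box overlap event passes the overlapping actor to LevelUp.
; LevelUp increments CurrentLevel only for a BP_Character and only until it reaches MaxLevel.
; Tick prints the current level on screen every frame, and the level drives nothing else here.
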(event OnComponentBeginOverlap(Box)
  (params (OverlappedComponent :type Primitive%20Component%20Object%20Reference) (OtherActor :type Actor%20Object%20Reference) (OtherComp :type Primitive%20Component%20Object%20Reference) (OtherBodyIndex :type Integer) (bFromSweep :type Boolean) (SweepResult :type Hit%20Result%20Structure%20%28by%20ref%29))
  (CallFunction|LevelUp OtherActor))

(event EventBeginPlay
  (Variables|Default|SetCurrentLevel 0)
  (Variables|Default|SetMaxLevel 2))

(event EventTick
  (params (DeltaSeconds :type Float%20%28single-precision%29))
  (Development|PrintString (Utilities|String|ToString(Integer) (Variables|Default|GetCurrentLevel)) true true "(R=0.000000,G=0.660000,B=1.000000,A=1.000000)" DeltaSeconds))

(fn ConstructionScript)

(fn LevelUp
  (params (Player :type Actor%20Object%20Reference))
  (Utilities|Casting|CastToBP_Character Player)
  (if (not (== (Variables|Default|GetCurrentLevel) (Variables|Default|GetMaxLevel)))
    (bind _result (Math|Integer|IncrementInt (Variables|Default|GetCurrentLevel))
      (:%20%20
        (Variables|Default|SetCurrentLevel _result)))))