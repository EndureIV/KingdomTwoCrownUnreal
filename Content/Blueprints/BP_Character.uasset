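; Player character Blueprint with single-axis movement along world X and a stamina-limited sprint, using Enhanced Input.
; BeginPlay adds the player mapping context and fills stamina.
; Sprint press raises walk speed and drains stamina in a looped retriggerable delay until release or exhaustion restores walk speed.
; Sprint release starts a similar loop that regenerates stamina to the maximum, without checking whether sprinting has resumed.
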(event Custom|Set%20Stamina
  (params (MaxStamina :type Float%20%28double-precision%29))
  (bind _output_get (Variables|Default|SetMaxStamina MaxStamina))
  (Variables|Default|SetCurrentStamina _output_get))

(event Custom|IncreaseStamina
  (params (Stamina%20Increase :type Float%20%28double-precision%29))
  (bind _maxstamina (Variables|Default|GetMaxStamina))
  ;[0.15 0.15 0.15 0.5] Regenerate Stamina
  (Variables|Default|SetCurrentStamina (Math|Float|Clamp(Float) (+ (Variables|Default|GetCurrentStamina) Stamina%20Increase) 0.0 _maxstamina))
  (if (== (Variables|Default|GetCurrentStamina) _maxstamina)
    (Variables|Default|SetCanRegenerateStamina false)
    (else
      (Variables|Default|SetCanRegenerateStamina true))))

(event Custom|UseStamina
  (params (StaminaPerUse :type Float%20%28double-precision%29))
  ;[0.15 0.15 0.15 0.5] Use Stamina
  (Variables|Default|SetCurrentStamina (Math|Float|Clamp(Float) (- (Variables|Default|GetCurrentStamina) StaminaPerUse) 0.0 (Variables|Default|GetMaxStamina)))
  (if (<= (Variables|Default|GetCurrentStamina) 0.0)
    (Variables|Default|SetIsSprinting false)
    (Variables|/Script/Engine.CharacterMovementComponent|SetMaxWalkSpeed (Variables|Character|GetCharacterMovement) (Variables|Default|GetWalkSpeed))))

(event Input|EnhancedActionEvents|EnhancedInputActionIA_MoveRight
  (params (ActionValue :type Float%20%28double-precision%29) (ElapsedSeconds :type Float%20%28double-precision%29) (TriggeredSeconds :type Float%20%28double-precision%29) (InputAction :type Input%20Action%20Object%20Reference :default "/Game/Blueprints/Inputs/IA_MoveRight.IA_MoveRight"))
  ;[0.15 0.15 0.15 0.5] Movement
  (Pawn|Input|AddMovementInput "1.000000,0.000000,0.000000" ActionValue false))

(event Input|EnhancedActionEvents|EnhancedInputActionIA_Sprint
  (params (ActionValue :type Boolean) (ElapsedSeconds :type Float%20%28double-precision%29) (TriggeredSeconds :type Float%20%28double-precision%29) (InputAction :type Input%20Action%20Object%20Reference :default "/Game/Blueprints/Inputs/IA_Sprint.IA_Sprint"))
  (bind _charactermovement (Variables|Character|GetCharacterMovement))
  ;[0.15 0.15 0.15 0.5] Sprint
  (:Started
    (Variables|Default|SetIsSprinting true)
    (Variables|/Script/Engine.CharacterMovementComponent|SetMaxWalkSpeed _charactermovement (Variables|Default|GetSprintSpeed) :!label _label)
    (Utilities|FlowControl|RetriggerableDelay 0.2)
    (CallFunction|UseStamina 5.0)
    (if (Variables|Default|GetIsSprinting)
      (goto _label)))
  (:Completed
    (Variables|Default|SetIsSprinting false)
    (Variables|/Script/Engine.CharacterMovementComponent|SetMaxWalkSpeed _charactermovement (Variables|Default|GetWalkSpeed) :!label _label_2)
    (Utilities|FlowControl|RetriggerableDelay 0.2)
    (CallFunction|IncreaseStamina 1e+01)
    (if (Variables|Default|GetCanRegenerateStamina)
      (goto _label_2))))

(event EventBeginPlay
  ;[0.15 0.15 0.15 0.5] Add Mapping contexte
  (bind _asplayer_controller (Utilities|Casting|CastToPlayerController (Pawn|GetController)))
  (Utilities|IsValid (PlayerController|LocalPlayerSubsystems|GetEnhancedInputLocalPlayerSubsystem _asplayer_controller)
    (:Is%20Valid
      (Input|AddMappingContext (PlayerController|LocalPlayerSubsystems|GetEnhancedInputLocalPlayerSubsystem _asplayer_controller) "/Game/Blueprints/Inputs/IMC_Player.IMC_Player" 0 "(bIgnoreAllPressedKeysUntilRelease=True,bForceImmediately=False,bNotifyUserSettings=False)")
      (CallFunction|SetStamina 1e+02))))

(fn ConstructionScript)