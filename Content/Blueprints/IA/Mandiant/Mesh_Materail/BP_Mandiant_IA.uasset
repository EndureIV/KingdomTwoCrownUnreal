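; Beggar AI ("Mandiant") that patrols between two fixed points and reacts to coins.
; BeginPlay loops chained AIMoveTo calls; a Target overlap with BP_Coins redirects movement to the coin's X at a fixed Y.
; A GrabCoin overlap calls LevelUp, fires the EDTest dispatcher and destroys actors.
; LevelUp and Addxp are empty; XP counting and level-based mesh swapping remain as unconnected test logic.
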(event OnComponentBeginOverlap(Target)
  (params (OverlappedComponent :type Primitive%20Component%20Object%20Reference) (OtherActor :type Actor%20Object%20Reference) (OtherComp :type Primitive%20Component%20Object%20Reference) (OtherBodyIndex :type Integer) (bFromSweep :type Boolean) (SweepResult :type Hit%20Result%20Structure%20%28by%20ref%29))
  (bind _asbp_coins (Utilities|Casting|CastToBP_Coins OtherActor))
  (CallFunction|Moveto (Transformation|GetWorldLocation (Variables|/Game/Blueprints/BP_Coins.BP_Coins_C|GetCoins _asbp_coins))))

(event OnComponentBeginOverlap(GrabCoin)
  (params (OverlappedComponent :type Primitive%20Component%20Object%20Reference) (OtherActor :type Actor%20Object%20Reference) (OtherComp :type Primitive%20Component%20Object%20Reference) (OtherBodyIndex :type Integer) (bFromSweep :type Boolean) (SweepResult :type Hit%20Result%20Structure%20%28by%20ref%29))
  (Utilities|Casting|CastToBP_Coins OtherActor)
  (CallFunction|LevelUp)
  (Actor|DestroyActor)
  (Default|CallEDTest)
  (Actor|DestroyActor))

(event Custom|Move%20to
  (params (Position :type Vector))
  (AI|AIMoveTo self (Math|Vector|MakeVector (.x Position) -1e+02 0.0) 0 5.0 false))

(event Custom|Add%20xp
  (params (Incremente :type Float%20%28double-precision%29))
  ;[0.15 0.006139 0 0.5] Teste changement etat
)

(event EventBeginPlay
  (Utilities|FlowControl|Sequence
    (:then_0
      (AI|AIMoveTo self "890.000000,-6.000000,21.000000" 0 5.0 false :!label _label
        (:OnSuccess
          (AI|AIMoveTo self "2395.000000,6.000000,21.000000" 0 5.0 false
            (:OnSuccess
              (goto _label))))))
    (:then_1
      (Variables|Default|SetLevel 0))))

(event Input|KeyboardEvents|F3
  (params (Key :type Key%20Structure :default "None"))
  ;[0.15 0.006139 0 0.5] Teste changement etat
)

(fn ConstructionScript)

(fn LevelUp
  (params (NewLevel :type Integer)))