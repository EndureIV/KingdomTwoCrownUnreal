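; BP_Lapin is a rabbit animal Blueprint with a rudimentary, apparently unfinished wandering behavior.
; On BeginPlay it issues one AIMoveTo with no wired destination, then after success or failure waits briefly and calls MoveToRandomLocation.
; That function picks a random reachable nearby point, then resets TargetLocation to zero without starting another move.
; A separate Moveto event issues AIMoveTo using the given X and a fixed Y.
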(event Custom|Move%20to
  (params (Position :type Vector))
  (AI|AIMoveTo self (Math|Vector|MakeVector (.x Position) -1e+02 0.0) 0 5.0 false))

(event EventBeginPlay
  (Variables|Default|SetTargetLocation "0, 0, 0")
  (AI|AIMoveTo self "0, 0, 0" 0 2e+01 false
    (:OnSuccess
      (Utilities|FlowControl|Delay 0.5))
    (:OnFail
      (Utilities|FlowControl|Delay 0.5)))
  (CallFunction|MovetoRandomLocation))

(fn ConstructionScript)

(fn FindRandomPosition
  (Variables|Default|SetTargetLocation (.RandomLocation (AI|Navigation|GetRandomReachablePointinRadius (Transformation|GetActorLocation) 1e+03 0 0)))
  (return))

(fn MovetoRandomLocation
  (CallFunction|FindRandomPosition)
  (Variables|Default|SetTargetLocation "0, 0, 0"))