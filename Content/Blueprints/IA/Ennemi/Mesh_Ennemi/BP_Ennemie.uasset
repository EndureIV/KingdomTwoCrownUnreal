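; BP_Ennemie is an NPC meant to progress through villager, worker and archer tiers by picking up coins, hammers and bows.
; LevelUp increments Level and swaps the skeletal mesh, while Lock and Moveto steer the AI toward items along X at fixed Y.
; The logic is unfinished: GrabCoin overlap calls an empty Etat, whose pickup logic is unwired, as are the patrol loop and Lock call.
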(event OnComponentBeginOverlap(Target)
  (params (OverlappedComponent :type Primitive%20Component%20Object%20Reference) (OtherActor :type Actor%20Object%20Reference) (OtherComp :type Primitive%20Component%20Object%20Reference) (OtherBodyIndex :type Integer) (bFromSweep :type Boolean) (SweepResult :type Hit%20Result%20Structure%20%28by%20ref%29))
  ;[0.15 0.07781 0 0.5] Deplacement NPC sur Arc/Marteau
)

(event OnComponentBeginOverlap(GrabCoin)
  (params (OverlappedComponent :type Primitive%20Component%20Object%20Reference) (OtherActor :type Actor%20Object%20Reference) (OtherComp :type Primitive%20Component%20Object%20Reference) (OtherBodyIndex :type Integer) (bFromSweep :type Boolean) (SweepResult :type Hit%20Result%20Structure%20%28by%20ref%29))
  ;[0.009562 0 0.15 0.5] Etat NPC
  (CallFunction|Etat OtherActor))

(event Custom|Move%20to
  (params (Position :type Vector))
  ;[0 0.1388 0.15 0.5] Ce deplace sur un axe
  (AI|AIMoveTo self (Math|Vector|MakeVector (.x Position) -1e+02 0.0) 0 5.0 false))

(event EventBeginPlay)

(fn ConstructionScript)

(fn LevelUp
  (params (NewLevel :type Integer))
  ;[0.15 0 0.00078 0.5] Etat PNJ
  (bind _result (Math|Integer|IncrementInt (Math|Integer|Clamp(Integer) (stale _output_get) 0 3))
    (:%20%20
      (bind _output_get (Variables|Default|SetLevel _result))
      (switch int _output_get
        (:1
          (Components|SkeletalMesh|SetSkeletalMeshAsset (Variables|Default|GetSkeletalMesh) "/Engine/Tutorial/SubEditors/TutorialAssets/Character/IA/T_Villagoie.T_Villagoie"))
        (:2
          (Components|SkeletalMesh|SetSkeletalMeshAsset (Variables|Default|GetSkeletalMesh) "/Engine/Tutorial/SubEditors/TutorialAssets/Character/IA/T_Ouvrier.T_Ouvrier"))
        (:3
          (Components|SkeletalMesh|SetSkeletalMeshAsset (Variables|Default|GetSkeletalMesh) "/Engine/Tutorial/SubEditors/TutorialAssets/Character/IA/T_Archet.T_Archet"))))))

(fn Etat
  (params (objet :type Object%20Object%20Reference))
  ;[0.15 0.15 0.15 0.5] etat pnj
)

(fn Lock
  (params (Objet :type Object%20Object%20Reference))
  (bind _asbp_coins (Utilities|Casting|CastToBP_Coins Objet))
  (if (== (Variables|Default|GetLevel) 0)
    (CallFunction|Moveto (Transformation|GetWorldLocation (Variables|/Game/Blueprints/BP_Coins.BP_Coins_C|GetCoins _asbp_coins)))
    (else
      (bind _asbp_hammer (Utilities|Casting|CastToBP_Hammer Objet))
      (if (== (Variables|Default|GetLevel) 2)
        (CallFunction|Moveto (Transformation|GetWorldLocation (Variables|/Game/Blueprints/BP_Tool.BP_Tool_C|GetTool _asbp_hammer)))
        (else
          (bind _asbp_arc (Utilities|Casting|CastToBP_Arc Objet))
          (if (== (Variables|Default|GetLevel) 3)
            (CallFunction|Moveto (Transformation|GetWorldLocation (Variables|/Game/Blueprints/BP_Tool.BP_Tool_C|GetTool _asbp_arc)))
            (else
              (return))))))))