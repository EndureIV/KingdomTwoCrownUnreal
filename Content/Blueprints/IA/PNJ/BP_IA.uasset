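; Recruitable NPC that wanders around a point until a coin turns it into a villager for the base.
; At level 0, the Checker overlap sends it sprinting along X on a fixed Y toward the coin and enables the Grabber.
; Grabbing consumes the coin, raises Level, swaps material, registers it with ABP_Base and walks it there faster.
; FunctionLevelUp only swaps to worker or archer material by tool class.
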(event OnComponentBeginOverlap(Checker)
  (params (OverlappedComponent :type Primitive%20Component%20Object%20Reference) (OtherActor :type Actor%20Object%20Reference) (OtherComp :type Primitive%20Component%20Object%20Reference) (OtherBodyIndex :type Integer) (bFromSweep :type Boolean) (SweepResult :type Hit%20Result%20Structure%20%28by%20ref%29))
  (CallFunction|FunctionChecker OtherActor))

(event OnComponentBeginOverlap(Grabber)
  (params (OverlappedComponent :type Primitive%20Component%20Object%20Reference) (OtherActor :type Actor%20Object%20Reference) (OtherComp :type Primitive%20Component%20Object%20Reference) (OtherBodyIndex :type Integer) (bFromSweep :type Boolean) (SweepResult :type Hit%20Result%20Structure%20%28by%20ref%29))
  (CallFunction|FunctionGrabber OtherActor))

(event Custom|EventPatrouille
  ;[0.15 0.15 0.15 0.5] Patrol
  (Utilities|FlowControl|Delay 0.2)
  (AI|AIMoveTo self (Math|Random|RandomPointinBoundingBox (Variables|Default|GetCenterWanderPos) (Math|Vector|MakeVector (Variables|Default|GetWanderRadius) 0.0 0.0)) 0 5.0 false :!label _label
    (:OnSuccess
      (goto _label))))

(event Custom|EventMoveTo
  (params (Pos :type Vector))
  ;[0.15 0.15 0.15 0.5] Move To
  (AI|AIMoveTo self (Math|Vector|MakeVector (.X (Math|Vector|BreakVector Pos)) -1e+02 0.0) 0 5.0 false
    (:OnSuccess
      _)
    (:OnFail
      _))
  (if (Utilities|PlayerLevel)
    (CallFunction|EventPatrouille)
    (CallFunction|FunctionSprint false)))

(event EventBeginPlay
  (Utilities|FlowControl|Sequence
    (:then_0
      (bind _returnvalue (Actor|GetActorOfClass "/Game/Blueprints/SSJ3_Batiments/ABP_Base.ABP_Base_C"))
      (Variables|Default|SetBaseRef _returnvalue))
    (:then_1
      (Variables|Default|SetLevel 0)
      (CallFunction|FunctionSprint false))
    (:then_2
      (CallFunction|EventPatrouille))))

(fn ConstructionScript)

(fn FunctionChecker
  (params (ActorHit :type Actor%20Object%20Reference))
  (if (Utilities|PlayerLevel)
    (bind _asbp_coins (Utilities|Casting|CastToBP_Coins ActorHit))
    (CallFunction|EventMoveto (Transformation|GetWorldLocation (Variables|/Game/Blueprints/BP_Coins.BP_Coins_C|GetCoins _asbp_coins)))
    (CallFunction|FunctionSprint true)
    (Variables|/Script/Engine.PrimitiveComponent|SetbGenerateOverlapEvents (Variables|Default|GetGrabber) true)))

(fn FunctionGrabber
  (params (ActorHit :type Actor%20Object%20Reference))
  (if (Utilities|PlayerLevel)
    (bind _asbp_coins (Utilities|Casting|CastToBP_Coins ActorHit))
    (Math|Integer|IncrementInt (Variables|Default|GetLevel)
      (:%20%20
        (Actor|DestroyActor _asbp_coins)
        (Default|CallEDRemovefromFirecampInfluence)
        (Rendering|Material|SetMaterial (Variables|Character|GetMesh) 0 "/Game/Materials/MI_Vilageois.MI_Vilageois")
        (CallFunction|EventMoveto (Transformation|GetWorldLocation (Variables|/Game/Blueprints/SSJ3_Batiments/ABP_Batiments.ABP_Batiments_C|GetBatimentLocation (Variables|Default|GetBaseRef))))
        (CallFunction|FunctionSprint false)
        (Variables|/Script/Engine.CharacterMovementComponent|SetMaxWalkSpeed (Variables|Character|GetCharacterMovement) (* (Variables|Default|GetBaseMS) 1.5))
        (Utilities|Array|Add (Variables|/Game/Blueprints/SSJ3_Batiments/ABP_Base.ABP_Base_C|GetVillageois (Variables|Default|GetBaseRef)) self)))))

(fn FunctionSprint
  (params (Sprint :type Boolean))
  (bind _charactermovement (Variables|Character|GetCharacterMovement))
  (if Sprint
    (Variables|/Script/Engine.CharacterMovementComponent|SetMaxWalkSpeed _charactermovement (* (Variables|Default|GetBaseMS) 2.0))
    (else
      (Variables|/Script/Engine.CharacterMovementComponent|SetMaxWalkSpeed _charactermovement (Variables|Default|GetBaseMS)))))

(fn FunctionLevelUp
  (params (ToolClass :type BP%20Tool%20Class%20Reference))
  (if (== ToolClass "/Game/Blueprints/BP_Hammer.BP_Hammer_C")
    (Rendering|Material|SetMaterial (Variables|Character|GetMesh) 0 "/Game/Materials/MI_Ouvrier.MI_Ouvrier")
    (else
      (Rendering|Material|SetMaterial (Variables|Character|GetMesh) 0 "/Game/Materials/MI_Archet.MI_Archet"))))