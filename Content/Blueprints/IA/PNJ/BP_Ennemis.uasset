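; Enemy NPC that walks to the base building, then retreats to the portal's spawn point and destroys itself.
; Box overlaps make it flee early when it touches coins or a level 2 or 3 AI unit.
; Hit workers and archers are sent to base as level 1 villagers, with the base's role lists updated.
; Walls it touches take damage while it is not fleeing.
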(event OnComponentBeginOverlap(Box)
  (params (OverlappedComponent :type Primitive%20Component%20Object%20Reference) (OtherActor :type Actor%20Object%20Reference) (OtherComp :type Primitive%20Component%20Object%20Reference) (OtherBodyIndex :type Integer) (bFromSweep :type Boolean) (SweepResult :type Hit%20Result%20Structure%20%28by%20ref%29))
  (CallFunction|EventCheckCollide OtherActor))

(event Custom|EventBackToBase
  (AI|AIMoveTo self (Math|Vector|MakeVector (.x (Transformation|GetWorldLocation (Variables|/Game/Blueprints/SSJ3_Batiments/ABP_Portal.ABP_Portal_C|GetSpawnLocation (Variables|Default|GetPortal)))) -1e+02 0.0) 0 5.0 false
    (:OnSuccess
      (Actor|DestroyActor))))

(event Custom|EventCheckCollide
  (params (ActorHit :type Actor%20Object%20Reference))
  (bind _baseref (Variables|Default|GetBaseRef))
  (bind _baseref_2 (Variables|Default|GetBaseRef))
  (bind _batimentlocation (Variables|/Game/Blueprints/SSJ3_Batiments/ABP_Batiments.ABP_Batiments_C|GetBatimentLocation _baseref))
  (bind _returnvalue (Transformation|GetWorldLocation _batimentlocation))
  (Utilities|FlowControl|Sequence
    (:then_0
      (if (not (Variables|Default|GetFleeing))
        (Utilities|Casting|CastToBP_Coins ActorHit)
        (Development|PrintString "Hello")
        (Variables|Default|SetFleeing true)
        (CallFunction|EventBacktoBase)))
    (:then_1
      (if (not (Variables|Default|GetFleeing))
        (bind _asbp_ia (Utilities|Casting|CastToBP_IA ActorHit))
        (switch int (Variables|/Game/Blueprints/IA/PNJ/BP_IA.BP_IA_C|GetLevel _asbp_ia)
          (:2
            (Variables|Default|SetFleeing true)
            (Default|EventMoveto _asbp_ia _returnvalue)
            (Variables|/Game/Blueprints/IA/PNJ/BP_IA.BP_IA_C|SetLevel _asbp_ia 1)
            (Default|FunctionLevelUp _asbp_ia)
            (Utilities|Array|Add (Variables|/Game/Blueprints/SSJ3_Batiments/ABP_Base.ABP_Base_C|GetVillageois _baseref_2) _asbp_ia)
            (Utilities|Array|RemoveItem (Variables|/Game/Blueprints/SSJ3_Batiments/ABP_Base.ABP_Base_C|GetOuvrier _baseref_2) _asbp_ia)
            (CallFunction|EventBacktoBase)
            (Audio|PlaySound2D "/Game/Sounds/Downgrade__1_.Downgrade__1_" 1.0 1.0 0.0 0 0))
          (:3
            (Variables|Default|SetFleeing true)
            (Default|EventMoveto _asbp_ia _returnvalue)
            (Variables|/Game/Blueprints/IA/PNJ/BP_IA.BP_IA_C|SetLevel _asbp_ia 1)
            (Default|FunctionLevelUp _asbp_ia)
            (Utilities|Array|Add (Variables|/Game/Blueprints/SSJ3_Batiments/ABP_Base.ABP_Base_C|GetVillageois _baseref) _asbp_ia)
            (Utilities|Array|RemoveItem (Variables|/Game/Blueprints/SSJ3_Batiments/ABP_Base.ABP_Base_C|GetArcher _baseref) _asbp_ia)
            (CallFunction|EventBacktoBase)
            (Audio|PlaySound2D "/Game/Sounds/Downgrade__1_.Downgrade__1_" 1.0 1.0 0.0 0 0)))))
    (:then_2
      (if (not (Variables|Default|GetFleeing))
        (bind _asabp_mur (Utilities|Casting|CastToABP_Mur ActorHit))
        (Default|EventTakeDamage _asabp_mur)))))

(event EventBeginPlay
  (|CallParentFunction)
  (bind _returnvalue (Actor|GetActorOfClass "/Game/Blueprints/SSJ3_Batiments/ABP_Portal.ABP_Portal_C"))
  (Variables|Default|SetPortal _returnvalue)
  (AI|AIMoveTo self (Math|Vector|MakeVector (.x (Transformation|GetWorldLocation (Variables|/Game/Blueprints/SSJ3_Batiments/ABP_Batiments.ABP_Batiments_C|GetBatimentLocation (Variables|Default|GetBaseRef)))) -1e+02 0.0) 0 5.0 false
    (:OnSuccess
      (CallFunction|EventBacktoBase))))

(fn ConstructionScript)