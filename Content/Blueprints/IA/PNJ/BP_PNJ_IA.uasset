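; NPC AI for a recruitable character that progresses from beggar to villager, worker and archer through coins, hammers and bows.
; Lock steers it toward the item matching its Level, Etat consumes the item, and LevelUp swaps the mesh material.
; Looping AIMoveTo chains form patrols, with villagers registering at BP_Base and targeting its walls.
; Event entry points and Etat are empty, leaving movement, pickup and XP logic disconnected.
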(event OnComponentBeginOverlap(Target)
  (params (OverlappedComponent :type Primitive%20Component%20Object%20Reference) (OtherActor :type Actor%20Object%20Reference) (OtherComp :type Primitive%20Component%20Object%20Reference) (OtherBodyIndex :type Integer) (bFromSweep :type Boolean) (SweepResult :type Hit%20Result%20Structure%20%28by%20ref%29))
  ;[0.15 0.07781 0 0.5] Deplacement NPC sur Coins/Mateau/Arc
)

(event OnComponentBeginOverlap(GrabCoin)
  (params (OverlappedComponent :type Primitive%20Component%20Object%20Reference) (OtherActor :type Actor%20Object%20Reference) (OtherComp :type Primitive%20Component%20Object%20Reference) (OtherBodyIndex :type Integer) (bFromSweep :type Boolean) (SweepResult :type Hit%20Result%20Structure%20%28by%20ref%29))
  ;[0.009562 0 0.15 0.5] Etat NPC
)

(event Custom|Move%20to
  (params (Position :type Vector))
  ;[0 0.1388 0.15 0.5] Ce deplace sur un axe
)

(event Custom|Add%20xp
  (params (Incremente :type Float%20%28double-precision%29))
  ;[0.15 0.006139 0 0.5] Teste changement etat
)

(event Custom|EventPatrouilleMandiant
  ;[0.15 0.15 0.15 0.5] Patrouille
)

(event Custom|EventPatrouilleVillageois)

(event EventBeginPlay
  ;[0.1475 0 0.15 0.5] Deplacement de base
)

(event Input|KeyboardEvents|F3
  (params (Key :type Key%20Structure :default "None"))
  ;[0.15 0.006139 0 0.5] Teste changement etat
)

(fn ConstructionScript)

(fn LevelUp
  ;[0.15 0 0.00078 0.5] Etat PNJ
  (bind _result (Math|Integer|IncrementInt (Variables|Default|GetLevel))
    (:%20%20
      (switch int _result
        (:1
          (Rendering|Material|SetMaterial (Variables|Default|GetSkeletalMesh) 0 "/Game/Materials/MI_Vilageois.MI_Vilageois"))
        (:2
          (Rendering|Material|SetMaterial (Variables|Default|GetSkeletalMesh) 0 "/Game/Materials/MI_Ouvrier.MI_Ouvrier"))
        (:3
          (Rendering|Material|SetMaterial (Variables|Default|GetSkeletalMesh) 0 "/Game/Materials/MI_Archet.MI_Archet"))))))

(fn Etat
  (params (objet :type Object%20Object%20Reference)))

(fn Lock
  (params (Objet :type Object%20Object%20Reference))
  (bind _asbp_coins (Utilities|Casting|CastToBP_Coins Objet)
    (:then
      (if (== (Variables|Default|GetLevel) 0)
        (CallFunction|Moveto (Transformation|GetWorldLocation (Variables|/Game/Blueprints/BP_Coins.BP_Coins_C|GetCoins _asbp_coins)))
        (else
          (bind _asbp_hammer (Utilities|Casting|CastToBP_Hammer Objet :!label _label)
            (:then
              (if (== (Variables|Default|GetLevel) 2)
                (CallFunction|Moveto (Transformation|GetWorldLocation (Variables|/Game/Blueprints/BP_Tool.BP_Tool_C|GetTool _asbp_hammer)))
                (return)
                (else
                  _)))
            (:CastFailed
              _))
          (bind _asbp_arc (Utilities|Casting|CastToBP_Arc Objet)
            (:then
              (if (== (Variables|Default|GetLevel) 3)
                (CallFunction|Moveto (Transformation|GetWorldLocation (Variables|/Game/Blueprints/BP_Tool.BP_Tool_C|GetTool _asbp_arc)))
                (return)
                (else
                  _)))
            (:CastFailed
              _))
          (return))))
    (:CastFailed
      (goto _label))))